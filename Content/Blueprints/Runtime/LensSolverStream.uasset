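; Cine camera Blueprint that solves lens calibration and distortion from a media stream.
; StartCalibration opens the URL; once opened, the stream plays and background corner-finding and calibration workers start.
; Event callbacks pass results and distortion maps to shared generic handlers, while Tick updates the solved lens from zoom level and focal lengths.
; Background image processors stop when the job finishes or play ends.
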(event EventTick
  (params (DeltaSeconds :type Float%20%28single-precision%29))
  (CallFunction|GenericSolvedLensTick (Variables|Default|GetInverseDistortionCorrection) (Variables|Default|GetZoomLevel) (.focalLengths (Utilities|Struct|BreakGenericLensSolverParameters (Variables|/Script/LensCalibrator.MediaStreamDataAsset|GetgenericLensSolverParameters (Variables|Default|GetInput)))) self))

(event EventOnGeneratedDistortionMaps
  (params (generatedCorrectionDistortionMap :type Texture%202D%20Object%20Reference) (generatedUnCorrectionDistortionMap :type Texture%202D%20Object%20Reference))
  (bind _input (Variables|Default|GetInput))
  (bind _genericlenssolverparameters (Variables|/Script/LensCalibrator.MediaStreamDataAsset|GetgenericLensSolverParameters _input))
  (bind (_zoomlevel _inversedistortioncorrection _cornerworkercount _calibrateworkercount _lensdistortionvolume _calibrationresults _focallengths _distortioncorrectionmaps _distortionuncorrectionmaps) (Utilities|Struct|BreakGenericLensSolverParameters _genericlenssolverparameters))
  (CallFunction|GenericHandleonGeneratedDistortionMap generatedCorrectionDistortionMap generatedUnCorrectionDistortionMap (Class|KismetSystemLibrary|MakeLiteralInteger 1) _distortioncorrectionmaps _distortionuncorrectionmaps _lensdistortionvolume))

(event EventOnReceiveCalibrationResult
  (params (calibrationResult :type Calibration%20Result%20Structure))
  (CallFunction|GenericHandleonRecieveCalibrationResult self calibrationResult (.calibrationResults (Utilities|Struct|BreakGenericLensSolverParameters (Variables|/Script/LensCalibrator.MediaStreamDataAsset|GetgenericLensSolverParameters (Variables|Default|GetInput))))))

(event EventOnFinishedJob
  (params (jobInfo :type Job%20Info%20Structure))
  (bind _input (Variables|Default|GetInput))
  (bind _genericlenssolverparameters (Variables|/Script/LensCalibrator.MediaStreamDataAsset|GetgenericLensSolverParameters _input))
  (bind (_zoomlevel _inversedistortioncorrection _cornerworkercount _calibrateworkercount _lensdistortionvolume _calibrationresults _focallengths) (Utilities|Struct|BreakGenericLensSolverParameters _genericlenssolverparameters))
  (Class|LensSolverBlueprintAPI|StopBackgroundImageprocessors)
  (CallFunction|GenericHandleonFinishedJob jobInfo self _calibrationresults _focallengths))

(event EventEndPlay
  (params (EndPlayReason :type EEndPlayReason%20Enum :default "Destroyed"))
  (Class|LensSolverBlueprintAPI|StopBackgroundImageprocessors))

(fn StartCalibration
  (bind _input (Variables|Default|GetInput))
  (bind _mediaplayer (Variables|/Script/LensCalibrator.MediaStreamDataAsset|GetmediaPlayer _input))
  (Media|MediaPlayer|BindEventtoOnMediaOpened _mediaplayer (EventDispatchers|CreateEvent :!event OnOpenedStream))
  (Class|MediaPlayer|OpenUrl _mediaplayer (Variables|/Script/LensCalibrator.MediaStreamDataAsset|Geturl (Variables|Default|GetInput))))

(fn OnOpenedStream
  (params (OpenedUrl :type String))
  (bind _input (Variables|Default|GetInput))
  (bind _genericlenssolverparameters (Variables|/Script/LensCalibrator.MediaStreamDataAsset|GetgenericLensSolverParameters _input))
  (bind (_zoomlevel _inversedistortioncorrection _cornerworkercount _calibrateworkercount) (Utilities|Struct|BreakGenericLensSolverParameters _genericlenssolverparameters))
  (Media|MediaPlayer|Play (Variables|/Script/LensCalibrator.MediaStreamDataAsset|GetmediaPlayer _input) :!class /Script/MediaAssets.MediaPlayer)
  (Class|LensSolverBlueprintAPI|StartBackgroundImageProcessors _cornerworkercount _calibrateworkercount)
  (Class|LensSolverBlueprintAPI|StartMediaStreamCalibration self (Variables|/Script/LensCalibrator.MediaStreamDataAsset|GetstartMediaStreamParameters _input)))