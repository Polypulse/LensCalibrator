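; Cine camera Blueprint that runs lens calibration from an array of texture/zoom pairs and applies the solved lens on Tick.
; StartCalibration launches background corner-finding and calibration workers, then submits the inputs as a one-time job.
; Receiver events delegate to shared generic handlers that collect results, focal lengths and distortion maps, with a distortion volume texture alongside.
; Tick feeds zoom level, focal lengths and inverse-correction setting to the generic solver; EndPlay stops the workers.
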(event EventOnGeneratedDistortionMaps
  (params (generatedCorrectionDistortionMap :type Texture%202D%20Object%20Reference) (generatedUnCorrectionDistortionMap :type Texture%202D%20Object%20Reference))
  (bind _input (Variables|Default|GetInput))
  (bind _genericlenssolverparameters (Variables|/Script/LensCalibrator.TextureFolderZoomPairDataAsset|GetgenericLensSolverParameters _input))
  (bind (_zoomlevel _inversedistortioncorrection _cornerworkercount _calibrateworkercount _lensdistortionvolume _calibrationresults _focallengths _distortioncorrectionmaps _distortionuncorrectionmaps) (Utilities|Struct|BreakGenericLensSolverParameters _genericlenssolverparameters))
  (CallFunction|GenericHandleonGeneratedDistortionMap generatedCorrectionDistortionMap generatedUnCorrectionDistortionMap (Utilities|Array|Length (Variables|/Script/LensCalibrator.TextureFolderZoomPairDataAsset|Getinputs _input)) _distortioncorrectionmaps _distortionuncorrectionmaps _lensdistortionvolume))

(event EventTick
  (params (DeltaSeconds :type Float%20%28single-precision%29))
  (bind _input (Variables|Default|GetInput))
  (bind _genericlenssolverparameters (Variables|/Script/LensCalibrator.TextureFolderZoomPairDataAsset|GetgenericLensSolverParameters _input))
  (bind (_zoomlevel _inversedistortioncorrection _cornerworkercount _calibrateworkercount _lensdistortionvolume _calibrationresults _focallengths) (Utilities|Struct|BreakGenericLensSolverParameters _genericlenssolverparameters))
  (CallFunction|GenericSolvedLensTick _inversedistortioncorrection _zoomlevel _focallengths self))

(event EventOnReceiveCalibrationResult
  (params (calibrationResult :type Calibration%20Result%20Structure))
  (CallFunction|GenericHandleonRecieveCalibrationResult self calibrationResult (.calibrationResults (Utilities|Struct|BreakGenericLensSolverParameters (Variables|/Script/LensCalibrator.TextureFolderZoomPairDataAsset|GetgenericLensSolverParameters (Variables|Default|GetInput))))))

(event EventOnFinishedJob
  (params (jobInfo :type Job%20Info%20Structure))
  (bind _input (Variables|Default|GetInput))
  (bind _genericlenssolverparameters (Variables|/Script/LensCalibrator.TextureFolderZoomPairDataAsset|GetgenericLensSolverParameters _input))
  (bind (_zoomlevel _inversedistortioncorrection _cornerworkercount _calibrateworkercount _lensdistortionvolume _calibrationresults _focallengths) (Utilities|Struct|BreakGenericLensSolverParameters _genericlenssolverparameters))
  (CallFunction|GenericHandleonFinishedJob jobInfo self _calibrationresults _focallengths))

(event EventEndPlay
  (params (EndPlayReason :type EEndPlayReason%20Enum :default "Destroyed"))
  (Class|LensSolverBlueprintAPI|StopBackgroundImageprocessors))

(fn StartCalibration
  (bind _input (Variables|Default|GetInput))
  (bind _input_2 (Variables|Default|GetInput))
  (bind _genericlenssolverparameters (Variables|/Script/LensCalibrator.TextureFolderZoomPairDataAsset|GetgenericLensSolverParameters _input_2))
  (bind (_zoomlevel _inversedistortioncorrection _cornerworkercount _calibrateworkercount) (Utilities|Struct|BreakGenericLensSolverParameters _genericlenssolverparameters))
  (Class|LensSolverBlueprintAPI|StartBackgroundImageProcessors _cornerworkercount _calibrateworkercount)
  (Class|LensSolverBlueprintAPI|OneTimeProcessArrayOfTextureFolderZoomPairs self (Variables|/Script/LensCalibrator.TextureFolderZoomPairDataAsset|Getinputs _input) (Variables|/Script/LensCalibrator.TextureFolderZoomPairDataAsset|GetoneTimeProcessParameters _input)))