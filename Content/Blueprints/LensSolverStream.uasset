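; Lens solver camera Blueprint that calibrates a cine camera's lens from a live media stream URL.
; StartCalibration plays the stream, starts background checkerboard-corner and calibration workers, then begins stream calibration with itself as event receiver.
; Job completion stops the workers and passes results to generic handlers, as generated distortion maps are routed toward a distortion volume texture.
; Tick applies the solved lens using zoom level, focal lengths and inverse distortion correction.
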(event EventTick
  (params (DeltaSeconds :type Float%20%28single-precision%29))
  (bind _genericlenssolverparameters (Variables|Default|GetGenericLensSolverParameters))
  (bind (_zoomlevel _inversedistortioncorrection _findcheckerboardworkercount _calibrateworkercount _lensdistortionvolume _calibrationresults _focallengths) (Utilities|Struct|BreakGenericLensSolverParameters _genericlenssolverparameters))
  (CallFunction|GenericSolvedLensTick _inversedistortioncorrection _zoomlevel _focallengths self))

(event EventOnGeneratedDistortionMaps
  (params (generatedCorrectionDistortionMap :type Texture%202D%20Object%20Reference) (generatedUnCorrectionDistortionMap :type Texture%202D%20Object%20Reference))
  (bind _genericlenssolverparameters (Variables|Default|GetGenericLensSolverParameters))
  (bind (_zoomlevel _inversedistortioncorrection _findcheckerboardworkercount _calibrateworkercount _lensdistortionvolume _calibrationresults _focallengths _distortioncorrectionmaps _distortionuncorrectionmaps) (Utilities|Struct|BreakGenericLensSolverParameters _genericlenssolverparameters))
  (CallFunction|GenericHandleonGeneratedDistortionMap generatedCorrectionDistortionMap generatedUnCorrectionDistortionMap (Class|KismetSystemLibrary|MakeLiteralInteger 1) _distortioncorrectionmaps _distortionuncorrectionmaps _lensdistortionvolume))

(event EventOnFinishedJob
  (params (jobInfo :type Job%20Info%20Structure))
  (bind _genericlenssolverparameters (Variables|Default|GetGenericLensSolverParameters))
  (bind (_zoomlevel _inversedistortioncorrection _findcheckerboardworkercount _calibrateworkercount _lensdistortionvolume _calibrationresults _focallengths) (Utilities|Struct|BreakGenericLensSolverParameters _genericlenssolverparameters))
  (Class|LensSolverBlueprintAPI|StopBackgroundImageprocessors)
  (CallFunction|GenericHandleonFinishedJob jobInfo self _calibrationresults _focallengths))

(event EventEndPlay
  (params (EndPlayReason :type EEndPlayReason%20Enum :default "Destroyed"))
  (Class|LensSolverBlueprintAPI|StopBackgroundImageprocessors))

(fn StartCalibration
  (bind _genericlenssolverparameters (Variables|Default|GetGenericLensSolverParameters))
  (bind (_zoomlevel _inversedistortioncorrection _findcheckerboardworkercount _calibrateworkercount) (Utilities|Struct|BreakGenericLensSolverParameters _genericlenssolverparameters))
  (Class|MediaPlayer|OpenUrl (Variables|Default|GetMediaPlayer) (Variables|Default|GetStreamURL))
  (Media|MediaPlayer|Play (Variables|Default|GetMediaPlayer) :!class /Script/MediaAssets.MediaPlayer)
  (Class|LensSolverBlueprintAPI|StartBackgroundImageProcessors _findcheckerboardworkercount _calibrateworkercount)
  (Class|LensSolverBlueprintAPI|StartMediaStreamCalibration self (Variables|Default|GetStartMediaStreamParameters)))