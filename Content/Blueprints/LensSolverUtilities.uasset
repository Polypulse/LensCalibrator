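; Utility functions for a lens solver, handling sampling and extraction of solved lens data.
; InterpolateBetweenValuesInFloatArray treats an array as an evenly spaced curve, linearly blending neighboring entries at a normalized position and returning zero when empty.
; It clamps the position just below one and adds an epsilon to avoid dividing by zero on exact indices.
; Two selector functions copy vertical FOV or aspect ratio from solved points into float arrays.
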(fn InterpolateBetweenValuesinFloatArray
  (params (FloatArray :type Array%20of%20Floats%20%28single-precision%29) (NormalizedInterpolationValue :type Float%20%28single-precision%29))
  (bind _returnvalue (Utilities|Array|Length FloatArray))
  (bind _returnvalue_2 (Math|Float|Clamp(Float) NormalizedInterpolationValue 0.0 0.9999))
  (bind _returnvalue_3 (- _returnvalue 1))
  (bind _returnvalue_4 (Math|Conversions|ToFloat(Integer) _returnvalue_3))
  (bind _returnvalue_5 (* _returnvalue_2 _returnvalue_4))
  (bind _returnvalue_6 (Math|Float|Floor _returnvalue_5))
  (bind _returnvalue_7 (Math|Float|Ceil _returnvalue_5))
  (bind _returnvalue_8 (Math|Conversions|ToFloat(Integer) _returnvalue_6))
  (bind _returnvalue_9 (Math|Conversions|ToFloat(Integer) _returnvalue_7))
  (bind _returnvalue_10 (- _returnvalue_9 _returnvalue_8))
  (if (== (Utilities|Array|Length FloatArray) 0)
    (return 0.0)
    (else
      (return (Math|Float|Lerp (Utilities|Array|Get(acopy) FloatArray _returnvalue_6) (Utilities|Array|Get(acopy) FloatArray (+ _returnvalue_6 1)) (/ (- _returnvalue_5 _returnvalue_8) (+ _returnvalue_10 (* (Math|Conversions|ToFloat(Boolean) (== _returnvalue_10 0.0)) 1e-05))))))))

(fn SelectVerticalFovValuesfromSolvedPointsArray
  (params (SolvedPoints :type Array%20of%20Calibration%20Result%20Structures))
  (Utilities|Array|Resize (LocalVariables|GetFloatArray) (Utilities|Array|Length SolvedPoints))
  (bind (_array_element _array_index) (Utilities|Array|ForEachLoopwithBreak SolvedPoints)
    (:LoopBody
      (Utilities|Array|SetArrayElem (LocalVariables|GetFloatArray) _array_index (.fovY (Utilities|Struct|BreakCalibrationResult _array_element))))
    (:Completed
      (return (LocalVariables|GetFloatArray)))))

(fn SelectAspectRatioValuesfromSolvedPointsArray
  (params (SolvedPoints :type Array%20of%20Calibration%20Result%20Structures))
  (Utilities|Array|Resize (LocalVariables|GetFloatArray) (Utilities|Array|Length SolvedPoints))
  (bind (_array_element _array_index) (Utilities|Array|ForEachLoopwithBreak SolvedPoints)
    (:LoopBody
      (Utilities|Array|SetArrayElem (LocalVariables|GetFloatArray) _array_index (.aspectRatio (Utilities|Struct|BreakCalibrationResult _array_element))))
    (:Completed
      (return (LocalVariables|GetFloatArray)))))