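; Camera calibration component that derives field of view from an array of textures paired with zoom levels.
; StartCalibration launches background corner-finding and calibration workers to process the pairs asynchronously, while Tick polls their queue.
; FinishedJob caches vertical FOVs and stops the workers; Tick then interpolates them by normalized zoom onto the owner's camera.
; DequeueSolvedPoints is empty, and the zoom-ordered insert into the cached results is unwired.
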(event EventTick
  (params (DeltaSeconds :type Float%20%28single-precision%29))
  ;[1 1 1] Ask the base class to check if we have any results in the queue from the workers.
  (Class|LensSolver|Poll)
  ;[1 1 1] After we are done processing, the following code lerps between calibration results using normalized zoom and sets camera parameters.
  (if (!= (Utilities|Array|Length (Variables|Default|GetCachedSolvedPoints)) 0)
    (if (not (Variables|Default|GetProcessing))
      (CallFunction|InterpolateBetweenFieldOfViewResults (Variables|Default|GetCachedVerticalFieldOfViewValues) (Variables|Default|GetZoomInterpolationValue)))))

(event EventDequeueSolvedPoints
  (params (solvedPoints :type Calibration%20Result%20Structure))
  ;[1 1 1] When a worker finishes processing an image, it gives the results back to us.
)

(event EventFinishedJob
  (params (jobInfo :type Job%20Info%20Structure))
  ;[1 1 1] This event lets us know when the workers are done processing all the images.
  ;[1 1 1] Here we are taking out of some of the individual struct members and packing them into their own arrays for easy access.
  (Variables|Default|SetCachedVerticalFieldOfViewValues (CallFunction|SelectVerticalFovValuesfromCalibrationResults (Variables|Default|GetCachedSolvedPoints)))
  ;[1 1 1] Stop background workers and flag within this blueprint that we are done processing.
  (Class|LensSolver|StopBackgroundImageprocessors)
  (Variables|Default|SetProcessing false))

(fn SortandStoreResult
  (params (InputPin :type Calibration%20Result%20Structure)))

(fn InterpolateBetweenFieldOfViewResults
  (params (VerticalFieldOfViews :type Array%20of%20Floats%20%28single-precision%29) (NormalizedInterpolationValue :type Float%20%28single-precision%29))
  (bind _returnvalue (Components|GetOwner))
  (bind _returnvalue_2 (Actor|GetComponentbyClass _returnvalue "/Script/Engine.CameraComponent"))
  (if (Utilities|IsValid _returnvalue_2)
    (Camera|SetFieldOfView _returnvalue_2 (CallFunction|InterpolateBetweenValuesinFloatArray VerticalFieldOfViews NormalizedInterpolationValue))))

(fn StartCalibration
  ;[1 1 1] For now, you need to explicility define how many workers you want to use and start them. We also need to explicility stop them because otherwise they will just continue to idle waiting for work.
  (Class|LensSolver|StartBackgroundImageProcessors (Variables|Default|GetFindConersWorkerCount) (Variables|Default|GetCalibrateWorkerCount))
  ;[1 1 1] Asynchronously process input textures each associated with a zoom level at the matching array index.
  (Class|LensSolver|OneTimeProcessArrayOfTextureZoomPairs (Variables|Default|GetInputs) (Variables|Default|GetInputOneTimeProcessParameters))
  (Variables|Default|SetProcessing true) ; Since we started this job, lets have a flag that describes that we are currently asynchronously processing.
)