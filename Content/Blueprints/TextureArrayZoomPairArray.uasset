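; Lens calibration component that calibrates from texture folder and zoom-level pairs using background workers, then drives the owner's CineCamera.
; Results are stored by zoom level, yielding focal lengths that Tick interpolates by ZoomLevel.
; On completion, the first result sets sensor size and generates distortion correction maps at hard-coded paths.
; A hard-coded test image runs through the correction map, and each returned image through the inverse map.
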(event EventTick
  (params (DeltaSeconds :type Float%20%28single-precision%29))
  (bind _returnvalue (Components|GetOwner))
  (bind _returnvalue_2 (Actor|GetComponentbyClass _returnvalue "/Script/CinematicCamera.CineCameraComponent"))
  (if (and (!= (Utilities|Array|Length (Variables|Default|GetCachedResults)) 0) (Utilities|IsValid _returnvalue_2))
    (CallFunction|ApplyInterpolatedFocalLengthtoCineCamera (Variables|Default|GetCachedFocalLengths) (Variables|Default|GetZoomLevel) _returnvalue_2)))

(event EventOnReceiveCalibrationResult
  (params (calibrationResult :type Calibration%20Result%20Structure))
  (CallFunction|InsertCalibrationResultbyZoomLevel calibrationResult (Variables|Default|GetCachedResults)))

(event EventOnFinishedJob
  (params (jobInfo :type Job%20Info%20Structure))
  (bind _cachedresults (Variables|Default|GetCachedResults))
  (bind _cachedresults_2 (Variables|Default|GetCachedResults))
  (bind _output (Utilities|Array|Get(acopy) _cachedresults_2))
  (bind (_baseparameters _success _fovx _fovy _focallengthmm _aspectratio _sensorsizemm _principalpixelpoint _resolution _perspectivematrix _distortioncoefficients) (Utilities|Struct|BreakCalibrationResult _output))
  (if (!= (Utilities|Array|Length _cachedresults) 0)
    (Variables|Default|SetCachedFocalLengths (CallFunction|SelectFocalLengthValuesfromCalibrationResults _cachedresults))
    (CallFunction|ApplySensorDimensionstoCineCamera _sensorsizemm (Actor|GetComponentbyClass (Components|GetOwner) "/Script/CinematicCamera.CineCameraComponent"))
    (Class|LensSolverBlueprintAPI|GenerateDistortionCorrectionMap self (Utilities|Struct|MakeDistortionCorrectionMapGenerationParameters (.zoomLevel (Utilities|Struct|BreakBaseParameters _baseparameters)) _resolution _principalpixelpoint _resolution "D:\\CalibrationResults\\DistortionCorrection\\Correction.png" "D:\\CalibrationResults\\DistortionCorrection\\InverseCorrection.png" _distortioncoefficients))))

(event EventOnDistortedImageCorrected
  (params (correctedDistortedImage :type Texture%202D%20Object%20Reference))
  (bind _self self)
  (if true
    (Class|LensSolverBlueprintAPI|DistortTexturewithTextureFile _self (Utilities|Struct|MakeDistortTextureWithTextureFileParams correctedDistortedImage "D:\\CalibrationResults\\DistortionCorrection\\InverseCorrection.png"))
    (else
      (Class|LensSolverBlueprintAPI|DistortTexturewithTextureFile _self (Utilities|Struct|MakeDistortTextureWithTextureFileParams correctedDistortedImage "D:\\CalibrationResults\\DistortionCorrection\\Correction.png")))))

(event EventOnGeneratedDistortionMap
  (params (generatedDistortionMap :type Texture%202D%20Object%20Reference))
  (bind _returnvalue (Class|KismetRenderingLibrary|ImportFileasTexture2D "R:\\Images\\zoom-0\\IMG_20200501_214808.jpg"))
  (Class|LensSolverBlueprintAPI|DistortTexturewithTextureFile self (Utilities|Struct|MakeDistortTextureWithTextureFileParams _returnvalue "D:\\CalibrationResults\\DistortionCorrection\\Correction.png")))

(event EventEndPlay
  (params (EndPlayReason :type EEndPlayReason%20Enum :default "Destroyed"))
  (Class|LensSolverBlueprintAPI|StopBackgroundImageprocessors))

(fn StartCalibration
  (Class|LensSolverBlueprintAPI|StartBackgroundImageProcessors (Variables|Default|GetFindCheckerboardWorkerCount) (Variables|Default|GetCalibrateWorkerCount))
  (Class|LensSolverBlueprintAPI|OneTimeProcessArrayOfTextureFolderZoomPairs self (Variables|Default|GetInput) (Variables|Default|GetInputOneTimeProcessParameter)))