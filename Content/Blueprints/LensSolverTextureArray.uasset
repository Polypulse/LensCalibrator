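; Lens solver component that calibrates a camera from checkerboard textures, each paired with a normalized zoom level.
; BeginPlay starts background workers on a one-time async job over the texture array.
; Tick polls for results, which are stored by matching zoom index, with failures printed.
; When the job finishes, it caches FOV and aspect ratio arrays, stops the workers, then interpolates both by zoom onto the owner's CameraComponent every tick.
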(event EventBeginPlay
  ;[1 1 1] For now, you need to explicility define how many workers you want to use and start them. We also need to explicility stop them because otherwise they will just continue to idle waiting for work.
  (Class|LensSolver|StartBackgroundImageProcessors (Variables|Default|GetWorkerCount))
  ;[1 1 1] Asynchronously process input textures each associated with a zoom level at the matching array index.
  (bind _ouptutjobinfo (Class|LensSolver|OneTimeProcessTexture2DArray (Variables|Default|GetCameraTextures) (Variables|Default|GetZoomValues) (Utilities|Struct|MakeOneTimeProcessParameters (Utilities|Struct|MakeWorkerParameters (Variables|Default|GetExhaustiveSearch) (Variables|Default|GetWriteDebugTextureToFile) (Variables|Default|GetDebugTextureFolderPath) (Variables|Default|GetWriteCalibrationResultsToFile) (Variables|Default|GetCalibrationResultsFolderPath)) (Variables|Default|GetCornerCount) (Variables|Default|GetSquareSizeInMM) (Variables|Default|GetResizeInputs) (Variables|Default|GetResizeResolution) (Variables|Default|GetFlipX) (Variables|Default|GetFlipY))))
  (Variables|Default|SetCurrentJobInfo _ouptutjobinfo) ; You can store a reference to the asynchronous job.
  (Variables|Default|SetProcessing true) ; Since we started this job, lets have a flag that describes that we are currently asynchronously processing.
)

(event EventTick
  (params (DeltaSeconds :type Float%20%28single-precision%29))
  ;[1 1 1] Ask the base class to check if we have any results in the queue from the workers.
  (Class|LensSolver|PollSolvedPoints)
  ;[1 1 1] After we are done processing, the following code lerps between calibration results using normalized zoom and sets camera parameters.
  (if (not (Variables|Default|GetProcessing))
    (CallFunction|InterpolateResultstoCamera (Variables|Default|GetCachedVerticalFieldOfViewValues) (Variables|Default|GetCachedAspectRatioValues) (Variables|Default|GetZoomInterpolationValue))))

(event EventDequeueSolvedPoints
  (params (solvedPoints :type Calibration%20Result%20Structure))
  ;[1 1 1] When a worker finishes processing an image, it gives the results back to us.
  (CallFunction|SortandStoreResult solvedPoints))

(event EventFinishedJob
  (params (jobInfo :type Job%20Info%20Structure))
  ;[1 1 1] This event lets us know when the workers are done processing all the images.
  ;[1 1 1] Here we are taking out of some of the individual struct members and packing them into their own arrays for easy access.
  (bind _verticalfieldofviews (CallFunction|SelectVerticalFovValuesfromSolvedPointsArray (Variables|Default|GetCachedSolvedPoints)))
  (Variables|Default|SetCachedVerticalFieldOfViewValues _verticalfieldofviews)
  (bind _verticalfieldofviews_2 (CallFunction|SelectAspectRatioValuesfromSolvedPointsArray (Variables|Default|GetCachedSolvedPoints)))
  (Variables|Default|SetCachedAspectRatioValues _verticalfieldofviews_2)
  ;[1 1 1] Stop background workers and flag within this blueprint that we are done processing.
  (Class|LensSolver|StopBackgroundImageprocessors)
  (Variables|Default|SetProcessing false))

(fn SortandStoreResult
  (params (InputPin :type Calibration%20Result%20Structure))
  (bind (_jobinfo _success _zoomlevel) (Utilities|Struct|BreakCalibrationResult InputPin))
  (bind (_array_element _array_index) (Utilities|Array|ForEachLoopwithBreak (Variables|Default|GetZoomValues) :!label _label)
    (:LoopBody
      (if (< (Math|Float|Absolute(Float) (- _array_element _zoomlevel)) 1e-05)
        (goto _label Break)))
    (:Completed
      (if _success
        _
        (else
          (Development|PrintString (Utilities|String|Append "Failed processing texture at index: " (Utilities|String|ToString(Integer) _array_index)) true true "(R=1.000000,G=0.000000,B=0.000000,A=1.000000)")))
      (Utilities|Array|SetArrayElem (Variables|Default|GetCachedSolvedPoints) _array_index InputPin true))))

(fn InterpolateResultstoCamera
  (params (VerticalFieldOfViews :type Array%20of%20Floats%20%28single-precision%29) (AspectRatios :type Array%20of%20Floats%20%28single-precision%29) (NormalizedInterpolationValue :type Float%20%28single-precision%29))
  (bind _returnvalue (Components|GetOwner))
  (bind _returnvalue_2 (Actor|GetComponentbyClass _returnvalue "/Script/Engine.CameraComponent"))
  (if (Utilities|IsValid _returnvalue_2)
    (bind _outputfloat (CallFunction|InterpolateBetweenValuesinFloatArray VerticalFieldOfViews NormalizedInterpolationValue))
    (Camera|SetFieldOfView _returnvalue_2 _outputfloat)
    (bind _outputfloat_2 (CallFunction|InterpolateBetweenValuesinFloatArray AspectRatios NormalizedInterpolationValue))
    (Class|CameraComponent|SetAspectRatio _returnvalue_2 _outputfloat_2)))